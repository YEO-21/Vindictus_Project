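; Knight enemy character Blueprint that raises a linked BPBars actor once the knight is dead.
; BeginPlay stores a target location 300 units above the bars.
; While IsDead is true, Tick sets the BPEnemyCharacter reference and calls SetBarsLocation.
; That function lifts the bars one unit per frame, independent of delta time, until the next step exactly equals the target.
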(event `self.ReceiveBeginPlay`
  (set `self.TargetLocation` (`KismetMathLibrary.MakeVector` (.x (`self.K2_GetActorLocation` (`self.BP_Bars`))) (.y (`self.K2_GetActorLocation` (`self.BP_Bars`))) (+ (.z (`self.K2_GetActorLocation` (`self.BP_Bars`))) 300.0))))

(event `self.ReceiveTick`
  (params (DeltaSeconds :type "Float (single-precision)"))
  (if (`self.IsDead`)
    (set `self.BP_EnemyCharacter` "BP_KnightCharacter_C")
    (`self.Set Bars Location`)))

(fn `Set Bars Location`
  (bind _bp_bars (`self.BP_Bars`))
  (bind _returnvalue (`KismetMathLibrary.MakeVector` (.x (`self.K2_GetActorLocation` _bp_bars)) (.y (`self.K2_GetActorLocation` _bp_bars)) (+ (.z (`self.K2_GetActorLocation` _bp_bars)) 1.0)))
  (if (not (== _returnvalue (`self.TargetLocation`)))
    (`self.K2_SetActorLocation` _bp_bars _returnvalue false false)))

(fn `UserConstructionScript`)