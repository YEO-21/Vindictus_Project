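; BP_ChickenCharacter is an enemy chicken character with an unfinished respawn mechanism.
; Tick calls Respawn whenever IsDead is set, which starts a seven-second timer on itself, prints a debug string and immediately clears the flag.
; The timed callback therefore does nothing unless IsDead is set again, and the node that would spawn a replacement chicken at the actor's transform is disconnected.
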(event `self.ReceiveBeginPlay`)

(event `self.ReceiveTick`
  (params (DeltaSeconds :type "Float (single-precision)"))
  (if (`self.IsDead`)
    (`self.Respawn`)))

(fn `Respawn`
  (if (`self.IsDead`)
    (`KismetSystemLibrary.K2_SetTimer` null "Respawn" 7.0)
    (`KismetSystemLibrary.PrintString` "Hello")
    (set `self.IsDead` false)))

(fn `UserConstructionScript`)