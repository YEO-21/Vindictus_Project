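; Dragon enemy character that plays a cinematic level sequence when it dies.
; Tick watches IsDead and starts SQ_CriticalAttack_Dragon once, guarded by IsPlayed.
; The sequence player binds play and finish events, and callback functions are provided to hide and show the top-level GameWidget.
; PlayDragonDeathAnimation is an empty stub.
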(event `self.ReceiveBeginPlay`)

(event `self.ReceiveActorBeginOverlap`
  (params (OtherActor :type "Actor Object Reference")))

(event `self.ReceiveTick`
  (params (DeltaSeconds :type "Float (single-precision)"))
  (if (and (`self.IsDead`) (not (`self.bIsPlayed`)))
    (set `self.BP_EnemyCharacter` "BP_DragonCharacter_C")
    (`self.Play Level Sequence`)))

(event `Play Level Sequence`
  ;[1 1 1] 데드 시퀀스 재생
  (bind (_outactor _returnvalue) (`LevelSequencePlayer.CreateLevelSequencePlayer` "/Game/Cinematic/SQ_CriticalAttack_Dragon.SQ_CriticalAttack_Dragon"))
  (add `MovieSceneSequencePlayer.OnFinished` _returnvalue (`|CreateDelegate` :!event `CALLBACK Show Game Widget`))
  (add `MovieSceneSequencePlayer.OnPlay` _returnvalue (`|CreateDelegate` :!event `CALLBACK Hide Game Widget`))
  (`MovieSceneSequencePlayer.Play` _returnvalue)
  (set `self.bIsPlayed` true))

(fn `CALLBACK Hide Game Widget`
  (bind _foundwidgets (`WidgetBlueprintLibrary.GetAllWidgetsOfClass` "/Script/soulproject.GameWidget"))
  (`GameWidget.HideAllWidget` (`|GetArrayItem` _foundwidgets)))

(fn `CALLBACK Show Game Widget`
  (bind _foundwidgets (`WidgetBlueprintLibrary.GetAllWidgetsOfClass` "/Script/soulproject.GameWidget"))
  (`GameWidget.ShowAllWidget` (`|GetArrayItem` _foundwidgets)))

(fn `Play Dragon Death Animation`)

(fn `UserConstructionScript`)