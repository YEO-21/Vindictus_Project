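; Interaction actor that shows a prompt widget in range and responds when the player interacts.
; Overlapping InteractionArea adds the InteractionF widget to the screen, and leaving removes it.
; Tick polls the player GameCharacter's IsInteractable flag, then shows the interaction widget, clears the flag and sets IsContainItem.
; Helper functions, not called here, remove the prompt and snap two target bridge meshes to hard-coded transforms.
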(event `self.ReceiveBeginPlay`)

(event `self.ReceiveTick`
  (params (DeltaSeconds :type "Float (single-precision)"))
  (bind _asgame_character (cast `GameCharacter` (`GameplayStatics.GetPlayerPawn` 0)))
  (if (`GameCharacter.isInteractable` _asgame_character)
    (bind _returnvalue (`|CreateWidget` "/Game/Blueprints/Widget/InteractionWidget/WidgetBP_Interaction.WidgetBP_Interaction_C"))
    (`UserWidget.AddToViewport` _returnvalue 0)
    (set `GameCharacter.isInteractable` false _asgame_character)
    (set `GameCharacter.isContainItem` true _asgame_character)))

(event `self.InteractionArea.OnComponentBeginOverlap`
  (params (OverlappedComponent :type "PrimitiveComponent Object Reference") (OtherActor :type "Actor Object Reference") (OtherComp :type "PrimitiveComponent Object Reference") (OtherBodyIndex :type Integer) (bFromSweep :type Boolean) (SweepResult :type "HitResult Structure (by ref)"))
  (bind _returnvalue (`|CreateWidget` "/Game/Blueprints/Widget/InteractionWidget/WidgetBP_InteractionF.WidgetBP_InteractionF_C"))
  (`UserWidget.AddToViewport` _returnvalue 0)
  (set `self.BP_InterationF` _returnvalue))

(event `self.InteractionArea.OnComponentEndOverlap`
  (params (OverlappedComponent :type "PrimitiveComponent Object Reference") (OtherActor :type "Actor Object Reference") (OtherComp :type "PrimitiveComponent Object Reference") (OtherBodyIndex :type Integer))
  (`/Engine/EditorBlueprintResources/StandardMacros.IsValid` (`self.BP_InterationF`)
    (:`Is Valid`
      (`Widget.RemoveFromParent` (stale `self.InteractionArea.OnComponentBeginOverlap` _returnvalue)))))

(fn `MoveBridgeAfterSQ`
  (`SceneComponent.K2_SetWorldTransform` (`StaticMeshActor.StaticMeshComponent` (`self.TargetStaticMesh1`)) (`KismetMathLibrary.MakeTransform` (1013.0 20.0 1980.0) (struct :`Pitch` 40.0)) false false)
  (`SceneComponent.K2_SetWorldTransform` (`StaticMeshActor.StaticMeshComponent` (`self.TargetStaticMesh2`)) (`KismetMathLibrary.MakeTransform` (988.0 12.0 1967.0) (struct :`Pitch` -40.0 :`Yaw` -180.0) (1.5 1.0 1.0)) false false))

(fn `RemoveWidget`
  (`GameViewportSubsystem.RemoveWidget` (subsystem `GameViewportSubsystem`) (`self.BP_InterationF`)))

(fn `UserConstructionScript`)